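; AI controller for enemies that starts the BT_Enemy behavior tree on BeginPlay.
; A looping one-second timer fires a Senses event, which is currently empty.
; Disconnected proximity logic would sphere-trace around the controlled pawn, ignoring BP_Lime actors, to update the LLClose blackboard key for player detection, but it never runs.
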(event Custom|Senses
  ;[1 1 1] If Player is close, move to player
)

(event EventTick
  (params (DeltaSeconds :type Float%20%28single-precision%29)))

(event EventBeginPlay
  (AI|RunBehaviorTree "/Game/AiEnemys/BT_Enemy.BT_Enemy")
  (Utilities|Time|SetTimerbyEvent (delegate Custom|Senses) 1.0 true))

(fn ConstructionScript)