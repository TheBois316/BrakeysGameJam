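; BP_Lemon is an AI-controlled lemon that the player can carry overhead and throw.
; PickUp toggles on the player's CarryLemon flag, either attaching it to the OverHead socket or launching it forward with one second of capsule physics.
; It mirrors the carried state into the LLClose blackboard key, clearing it after the throw settles.
; Overlapping a BP_Area prints a death message and reveals BP_Boat with collision enabled.
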(event Collision|EventActorBeginOverlap
  (params (OtherActor :type Actor%20Object%20Reference))
  (Utilities|Casting|CastToBP_Area OtherActor)
  (Development|PrintString "Dead")
  (bind _returnvalue (Actor|GetActorOfClass "/Game/ObjectsInLevels/Boat/BP_Boat.BP_Boat_C"))
  (Collision|SetActorEnableCollision _returnvalue true)
  (Rendering|SetActorHiddenInGame _returnvalue false))

(event EventPickUp
  (bind _capsulecomponent (Variables|Collision|GetCapsuleComponent))
  (bind _asbp_player (Utilities|Casting|CastToBP_Player (Game|GetPlayerCharacter 0)))
  (if (Variables|/Game/TopDownBP/Blueprints/BP_Player.BP_Player_C|GetbCarryLemon _asbp_player)
    (Variables|/Game/TopDownBP/Blueprints/BP_Player.BP_Player_C|SetbCarryLemon _asbp_player false)
    (Transformation|DetachFromActor "KeepWorld" "KeepWorld" "KeepWorld")
    (Collision|SetActorEnableCollision true)
    (Physics|SetSimulatePhysics _capsulecomponent true)
    (Physics|SetPhysicsLinearVelocity _capsulecomponent (* (Transformation|GetActorForwardVector _asbp_player) 1e+03) true "None")
    (Development|PrintString "Hello")
    (Utilities|FlowControl|Delay 1.0)
    (Physics|SetSimulatePhysics _capsulecomponent false)
    (AI|Components|Blackboard|SetValueasBool (AI|GetBlackboard (Pawn|GetController)) (Utilities|Name|MakeLiteralName "LLClose") false)
    (else
      (Variables|/Game/TopDownBP/Blueprints/BP_Player.BP_Player_C|SetbCarryLemon _asbp_player true)
      (Collision|SetActorEnableCollision false)
      (Transformation|AttachComponentToComponent (Variables|Character|GetMesh _asbp_player) "OverHead" "SnapToTarget" "KeepRelative" "KeepRelative" true)
      (AI|Components|Blackboard|SetValueasBool (AI|GetBlackboard (Pawn|GetController)) (Utilities|Name|MakeLiteralName "LLClose") true))))

(fn ConstructionScript)

(fn Use
  (return))